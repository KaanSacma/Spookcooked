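; Villager AI that wanders between random patrol points, carries a random monster-type Fear and destroys itself when its WaitTime runs out.
; A box overlap compares the other actor with the first found zombie, skeleton, ghost or vampire.
; Zombie and skeleton require a matching Fear, while ghost and vampire always count.
; A hit destroys monster and villager and increments the HUD score.
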(event `self.ReceiveBeginPlay`
  (set `self.Fear` (cast `/Game/Blueprints/MonsterType` (`KismetMathLibrary.Conv_IntToByte` (`KismetMathLibrary.RandomIntegerInRange` 0 (- (enumcount `/Game/Blueprints/MonsterType`) 1)))))
  (`self.PathPatrol`))

(event `self.ReceiveTick`
  (params (DeltaSeconds :type "Float (single-precision)"))
  (`self.CountdownVillagerLife`)
  (if (<= (`self.WaitTime`) 0.0)
    (`self.K2_DestroyActor`)))

(event `PathPatrol`
  (`|AIMoveTo` self (`|GetArrayItem` (`self.PatrolLocation`) (`KismetMathLibrary.RandomInteger` (`KismetArrayLibrary.Array_Length` (`self.PatrolLocation`)))) null 100.0
    (:`OnSuccess`
      (`KismetSystemLibrary.Delay` (`KismetMathLibrary.RandomFloatInRange` 1.0 3.0))
      (`self.PathPatrol`))
    (:`OnFail`
      (`self.PathPatrol`))))

(event `CountdownVillagerLife`
  (set `self.WaitTime` (`KismetMathLibrary.FClamp` (- (`self.WaitTime`) (`GameplayStatics.GetWorldDeltaSeconds`)) 0.0 (`self.WaitTime`))))

(event `self.Box.OnComponentBeginOverlap`
  (params (OverlappedComponent :type "PrimitiveComponent Object Reference") (OtherActor :type "Actor Object Reference") (OtherComp :type "PrimitiveComponent Object Reference") (OtherBodyIndex :type Integer) (bFromSweep :type Boolean) (SweepResult :type "HitResult Structure (by ref)"))
  (bind _returnvalue (`GameplayStatics.GetActorOfClass` "/Game/Blueprints/AI/Zombie/AI_Zombie.AI_Zombie_C"))
  (if (== OtherActor _returnvalue)
    (if (`|EnumEquality` (`self.Fear`) "NewEnumerator1")
      (`self.K2_DestroyActor` OtherActor :!label _label)
      (bind _foundwidgets (`WidgetBlueprintLibrary.GetAllWidgetsOfClass` "/Game/Interface/UIGameHud.UIGameHud_C"))
      (`/Game/Interface/UIGameHud.IncrementScoreValue` (`|GetArrayItem` _foundwidgets))
      (`self.K2_DestroyActor`))
    (else
      (bind _returnvalue_2 (`GameplayStatics.GetActorOfClass` "/Game/Blueprints/AI/Skeleton/AI_Skeleton.AI_Skeleton_C"))
      (if (== _returnvalue_2 OtherActor)
        (if (`|EnumEquality` (`self.Fear`) "NewEnumerator2")
          (goto _label))
        (else
          (bind _returnvalue_3 (`GameplayStatics.GetActorOfClass` "/Game/Blueprints/AI/Ghost/AI_Ghost.AI_Ghost_C"))
          (if (== _returnvalue_3 OtherActor)
            (if true
              (goto _label))
            (else
              (bind _returnvalue_4 (`GameplayStatics.GetActorOfClass` "/Game/Blueprints/AI/Vampire/AI_Vampire.AI_Vampire_C"))
              (if (== _returnvalue_4 OtherActor)
                (if true
                  (goto _label))))))))))

(fn `UserConstructionScript`)