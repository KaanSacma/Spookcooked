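; BP_ZombieSpawner periodically spawns IT_ShovelDirt pawns at its Billboard's location while their world count is below MaxShovelDirt.
; Each Tick counts them with GetAllActorsOfClass and, if under the cap, adds delta time to DelayTimer.
; When the timer reaches MaxDelaySpawn, it calls SpawnSystemAtLocation and SpawnAIFromClass there, then resets the timer.
; The cap covers all such actors in the world, and the timer pauses while it is met.
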(event `self.ReceiveTick`
  (params (DeltaSeconds :type "Float (single-precision)"))
  (bind _returnvalue (`SceneComponent.K2_GetComponentLocation` (`self.Billboard`)))
  (bind _outactors (`GameplayStatics.GetAllActorsOfClass` "/Game/Blueprints/Interactions/ShovelDirt/IT_ShovelDirt.IT_ShovelDirt_C"))
  (if (< (`KismetArrayLibrary.Array_Length` _outactors) (`self.MaxShovelDirt`))
    (bind _output (`self.Increment Delay` (`self.DelayTimer`) (`GameplayStatics.GetWorldDeltaSeconds`)))
    (bind _output_get (set `self.DelayTimer` _output))
    (`/Engine/EditorBlueprintResources/StandardMacros.CompareFloat` _output_get (`self.MaxDelaySpawn`)
      (:`>`
        _)
      (:`==`
        _))
    (`NiagaraFunctionLibrary.SpawnSystemAtLocation` null _returnvalue)
    (`AIBlueprintHelperLibrary.SpawnAIFromClass` "/Game/Blueprints/Interactions/ShovelDirt/IT_ShovelDirt.IT_ShovelDirt_C" null _returnvalue (struct) false null)
    (set `self.DelayTimer` 0.0)))

(fn `Increment Delay`
  (params (InputA :type "Float (double-precision)") (InputB :type "Float (double-precision)"))
  (returns (Output :type "Float (double-precision)"))
  (return (+ InputA InputB)))

(fn `UserConstructionScript`)