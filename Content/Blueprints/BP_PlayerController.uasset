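; Player controller that shows the mouse cursor and aims the controlled pawn at it.
; Each tick it projects the pawn's location to screen space and computes a look-at rotation from that point to the mouse position.
; The rotation is worked out in flat screen coordinates with no world trace, then handed to the pawn through SetRotationMessage.
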(event `self.ReceiveBeginPlay`
  (set `self.bShowMouseCursor` true))

(event `self.ReceiveTick`
  (params (DeltaSeconds :type "Float (single-precision)"))
  (bind (_locationx _locationy) (`self.GetMousePosition`))
  (message `/Game/Blueprints/BPI_Character.SetRotation` (`self.K2_GetPawn`) (`KismetMathLibrary.FindLookAtRotation` (`KismetMathLibrary.Conv_Vector2DToVector` (`GameplayStatics.ProjectWorldToScreen` self (`self.K2_GetActorLocation` (`self.K2_GetPawn`)))) (`KismetMathLibrary.MakeVector` _locationx _locationy))))

(fn `UserConstructionScript`)