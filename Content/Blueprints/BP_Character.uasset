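; Player character Blueprint with camera-relative movement and a zoomable spring-arm camera, driven by Enhanced Input.
; Movement input follows the control rotation's yaw, while zoom input adjusts the spring arm length within min and max limits.
; Tick turns the actor toward a Target rotation at constant speed, using RInterpToConstant.
; A SetRotation event snaps actor yaw to a given rotation, offset by the spring arm's relative yaw.
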(event `self.ReceiveTick`
  (params (DeltaSeconds :type "Float (single-precision)"))
  (`self.K2_SetActorRotation` (`KismetMathLibrary.RInterpTo_Constant` (`self.K2_GetActorRotation`) (`self.Target`) DeltaSeconds 180.0)))

(event `/Game/Blueprints/BPI_Character.SetRotation`
  (params (Rotator :type "Rotator Structure"))
  (bind (_relativerotation_roll _relativerotation_pitch _relativerotation_yaw) (`KismetMathLibrary.BreakRotator` (`SceneComponent.RelativeRotation` (`self.SpringArm`))))
  (`self.K2_SetActorRotation` (`KismetMathLibrary.MakeRotator` 0.0 0.0 (- Rotator_Yaw _relativerotation_yaw))))

(event `EnhancedInput|/Game/Blueprints/Input/IA_Movement`
  (params (ActionValue :type "Vector2D Structure") (ElapsedSeconds :type "Float (double-precision)") (TriggeredSeconds :type "Float (double-precision)") (InputAction :type "InputAction Object Reference" :default "/Game/Blueprints/Input/IA_Movement.IA_Movement"))
  (bind (_returnvalue_roll _returnvalue_pitch _returnvalue_yaw) (`KismetMathLibrary.BreakRotator` (`self.GetControlRotation`)))
  (bind _returnvalue (`KismetMathLibrary.MakeRotator` 0.0 0.0 _returnvalue_yaw))
  (:`Triggered`
    (`|ExecutionSequence`
      (:`then_0`
        (`self.AddMovementInput` (`KismetMathLibrary.GetForwardVector` _returnvalue) ActionValue_Y))
      (:`then_1`
        (`self.AddMovementInput` (`KismetMathLibrary.GetRightVector` _returnvalue) ActionValue_X)))))

(event `EnhancedInput|/Game/Blueprints/Input/IA_Zoom`
  (params (ActionValue :type "Float (double-precision)") (ElapsedSeconds :type "Float (double-precision)") (TriggeredSeconds :type "Float (double-precision)") (InputAction :type "InputAction Object Reference" :default "/Game/Blueprints/Input/IA_Zoom.IA_Zoom"))
  (bind _springarm (`self.SpringArm`))
  (:`Triggered`
    (set `SpringArmComponent.TargetArmLength` (`KismetMathLibrary.FClamp` (- (`SpringArmComponent.TargetArmLength` _springarm) ActionValue) (`self.MinZoomCamera`) (`self.MaxZoomCamera`)) _springarm)))

(fn `UserConstructionScript`)